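; BP_GameModeMenu is a menu game mode Blueprint whose only event graph logic is disconnected, so none of it runs.
; The dormant sequence disables touch controller sticks and sets game-only input on levels other than the menu map.
; It also prints device orientation and toggles the FPS stat display.
; The construction script is empty.
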(fn `UserConstructionScript`)