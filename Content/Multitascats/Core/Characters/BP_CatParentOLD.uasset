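; Parent cat character (named OLD) for an auto-runner, steered sideways by left-screen swipes or a Left/Right axis.
; Overlapped actors report their type to set the state: obstacles kill and restart the level after a delay, floors enable moving, ramps set a ramp state.
; Tick applies GameInstance forward speed and eases yaw and sideways drift back after touch release.
; Ramp movement is disconnected, right-screen touch only prints, and touch-on-character detection is unfinished.
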(event `self.ReceiveBeginPlay`
  ;[0 1 0.5961 1 200] BEGIN PLAY
  ;;[1 1 1] BEGIN PLAY
  (`|ExecutionSequence`
    (:`then_0`
      ;;[1 1 1] Game Instance and Game Mode REF
      (bind _asbp_game_instance (cast `/Game/Multitascats/Core/GameInstance/BP_GameInstance` (`GameplayStatics.GetGameInstance`)))
      (set `self.GameInstance_REF` _asbp_game_instance)
      (bind _asbp_game_mode (cast `/Game/Multitascats/Core/GameModes/BP_GameMode` (`GameplayStatics.GetGameMode`)))
      (set `self.GameMode_REF` _asbp_game_mode))
    (:`then_1`
      ;;[1 1 1] Set Horizontal Swipe Speed
      (`self.SetHorizontalSwipeSpeed`))))

(event `self.ReceiveTick`
  (params (DeltaSeconds :type "Float (single-precision)"))
  (bind (_returnvalue_x _returnvalue_y _returnvalue_z) (`KismetMathLibrary.BreakVector` (`self.GetVelocity`)))
  (bind _returnvalue (`self.K2_GetActorRotation`))
  (bind _returnvalue_2 (`self.GetVelocity`))
  (bind _returnvalue_3 (`self.K2_GetActorRotation`))
  (bind (_returnvalue_x_2 _returnvalue_y_2 _returnvalue_z_2) (`KismetMathLibrary.BreakVector` (`self.GetVelocity`)))
  ;[1 1 1] EVENT TICK
  (set `self.deltaSeconds` DeltaSeconds)
  (`KismetSystemLibrary.PrintString` (`KismetStringLibrary.Conv_BoolToString` (`NavMovementComponent.IsFalling` (`self.CharacterMovement`))))
  ;[1 1 1] Do Everything if Character is Alive
  (if (not (`|EnumEquality` (`self.characterState`) "NewEnumerator0"))
    (`|ExecutionSequence`
      (:`then_0`
        ;[1 1 1] Move Forward - Set X Velocity to Max Forward Speed
        (if (`|EnumEquality` (`self.characterState`) "NewEnumerator3")
          (set `MovementComponent.Velocity` (`KismetMathLibrary.MakeVector` (`/Game/Multitascats/Core/GameInstance/BP_GameInstance.forwardSpeed` (`self.GameInstance_REF`)) _returnvalue_y _returnvalue_z) (`self.CharacterMovement`))))
      (:`then_1`
        ;[1 1 1] Reset Rotation after Finger Released from Touch Input
        (if (`self.bFingerReleased`)
          (`self.K2_SetActorRotation` (`KismetMathLibrary.RInterpTo` _returnvalue_3 (`KismetMathLibrary.MakeRotator` (.roll _returnvalue_3) (.pitch _returnvalue_3)) (`self.deltaSeconds`) 10.0))
          ;[1 1 1] Reduce Y Velocity to prevent Character from Sliding Left or Right after Finger Released from Touch Input
          (set `MovementComponent.Velocity` (`KismetMathLibrary.VInterpTo` _returnvalue_2 (`KismetMathLibrary.MakeVector` (.x _returnvalue_2) 0.0 (.z _returnvalue_2)) (`self.deltaSeconds`) 10.0) (`self.CharacterMovement`))))
      (:`then_2`
        ;[1 1 1] If Character is On a Ramp adjust Rotation and Movement Speed
        (if (`|EnumEquality` (`self.characterState`) "NewEnumerator4")
          _))
      (:`then_3`
        ;[1 1 1] If Character starts Falling, Reset Rotation
        (if (`|EnumEquality` (`self.characterState`) "NewEnumerator1")
          ;[1 1 1] Adjust Forward Speed
          (set `MovementComponent.Velocity` (`KismetMathLibrary.MakeVector` (`/Game/Multitascats/Core/GameInstance/BP_GameInstance.forwardSpeed` (`self.GameInstance_REF`)) _returnvalue_y_2 _returnvalue_z_2) (`self.CharacterMovement`))
          ;[1 1 1] Reset Rotation
          (`self.K2_SetActorRotation` (`KismetMathLibrary.RInterpTo` _returnvalue (`KismetMathLibrary.MakeRotator` (.roll _returnvalue) 0.0 (.yaw _returnvalue)) (`self.deltaSeconds`) 10.0)))))))

(event `self.CatCollisionBox.OnComponentBeginOverlap`
  (params (OverlappedComponent :type "PrimitiveComponent Object Reference") (OtherActor :type "Actor Object Reference") (OtherComp :type "PrimitiveComponent Object Reference") (OtherBodyIndex :type Integer) (bFromSweep :type Boolean) (SweepResult :type "HitResult Structure (by ref)"))
  (bind _mesh (`self.Mesh`))
  (bind _overlappedactor_ref (`self.OverlappedActor_REF`))
  ;[0 1 0.5961 1 200] Overlap Events
  ;;[1 1 1] On Overlap
  ;;[1 1 1] Check if Overlapped Actor exists and is the same object in case overlap fires again. If True -> Dont execute the code again because state is already set
  (`/Engine/EditorBlueprintResources/StandardMacros.IsValid` _overlappedactor_ref
    (:`Is Valid`
      (if (not (== _overlappedactor_ref OtherActor))
        (bind _output_get (set `self.OverlappedActor_REF` OtherActor :!label _label))
        (bind (_isobstacle _isramp _isfloor) (message `/Game/Multitascats/Core/Interfaces/BPI_ActorTypes.Actor Type` _output_get))
        (`|ExecutionSequence`
          (:`then_0`
            ;;[1 1 1] is Obstacle and State is not already Dead
            (if (and (not (`|EnumEquality` (`self.characterState`) "NewEnumerator0")) _isobstacle)
              ;;[0 0 0] DEATH STATE
              (set `self.characterState` "NewEnumerator0")
              ;;;[1 1 1] Change Collision to prevent Ragdoll Bugs (Set Physics True)
              (`PrimitiveComponent.SetCollisionResponseToChannel` _mesh "ECC_WorldStatic" "ECR_Block")
              (`PrimitiveComponent.SetCollisionResponseToChannel` _mesh "ECC_WorldDynamic" "ECR_Block")
              ;;;[1 1 1] Disable Input and Set Velocity to 0
              (`self.DisableInput` (`GameplayStatics.GetPlayerController` 0))
              (set `MovementComponent.Velocity` (0.0 0.0 0.0) (`self.CharacterMovement`))
              ;;;[1 1 1] Level Restart after Delay
              (`KismetSystemLibrary.Delay` 2.5)
              (`/Game/Multitascats/Core/GameModes/BP_GameMode.RestartCurrentLevel` (`self.GameMode_REF`))))
          (:`then_1`
            ;;[1 1 1] is Ramp
            (if _isramp
              ;;[1 1 1] RAMP STATE
              (set `self.characterState` "NewEnumerator4")))
          (:`then_2`
            ;;[1 1 1] is Floor and State is not already isMoving
            (if (and (not (`|EnumEquality` (`self.characterState`) "NewEnumerator3")) _isfloor)
              ;;[1 1 1] MOVING STATE
              (set `self.characterState` "NewEnumerator3"))))))
    (:`Is Not Valid`
      (goto _label))))

(event `InputTouch`
  (params (Location :type "Vector Structure") (FingerIndex :type "ETouchIndex Enum"))
  (bind _returnvalue_x (`KismetMathLibrary.BreakVector2D` (`WidgetLayoutLibrary.GetViewportSize`)))
  (bind _returnvalue (`KismetMathLibrary.Abs` (- (`self.horizontalTouchDirectionChange`) (`self.horizontalTouchDirectionStart`))))
  (bind _returnvalue_2 (`KismetMathLibrary.GetRightVector` (`KismetMathLibrary.MakeRotator` 0.0 0.0 (.yaw (`self.GetControlRotation`)))))
  ;[0 1 0.5961 1 200] INPUT TOUCH
  (:`Pressed`
    ;;[1 1 1] InputTouch Pressed Initialize Variables
    (`|ExecutionSequence`
      (:`then_0`
        (set `self.InputLocationX` Location_X))
      (:`then_1`
        (set `self.InputLocationY` Location_Y))
      (:`then_2`
        (set `self.horizontalTouchDirectionStart` (`self.InputLocationX`)))
      (:`then_3`
        (set `self.verticalTouchDirectionStart` (`self.InputLocationY`)))
      (:`then_4`
        (set `self.bFingerReleased` false))))
  (:`Released`
    ;;[1 1 1] InputTouch Release
    (set `self.bFingerReleased` true))
  (:`Moved`
    (`|ExecutionSequence`
      (:`then_0`
        ;;[1 1 1] InputTouch Moved Initialize Change Variables
        (set `self.InputLocationX` Location_X))
      (:`then_1`
        (set `self.InputLocationY` Location_Y))
      (:`then_2`
        (set `self.horizontalTouchDirectionChange` (`self.InputLocationX`)))
      (:`then_3`
        (set `self.verticalTouchDirectionChange` (`self.InputLocationY`)))
      (:`then_4`
        ;;[1 1 1] True == LEFT SCREEN || False == RIGHT SCREEN
        (if (<= (`self.InputLocationX`) (/ _returnvalue_x 2.0))
          ;;[1 1 1] LEFT SCREEN SIDE
          (if (not (< (`self.horizontalTouchDifference`) _returnvalue))
            ;;;[1 1 1] If Swipe Direction Changes Set New Starting Point For Calculation
            (set `self.horizontalTouchDirectionStart` (`self.horizontalTouchDirectionChange`)))
          (set `self.horizontalTouchDifference` _returnvalue)
          (if (< (`self.horizontalTouchDirectionStart`) (`self.horizontalTouchDirectionChange`))
            ;;;[1 1 1] Swipe Right Direction
            (`self.AddMovementInput` _returnvalue_2)
            (elif (> (`self.horizontalTouchDirectionStart`) (`self.horizontalTouchDirectionChange`))
              ;;;[1 1 1] Swipe Left Direction
              (`self.AddMovementInput` _returnvalue_2 -1.0)))
          (else
            ;;[1 1 1] Right Screen Side - Up === True and Down === False
            (`KismetSystemLibrary.PrintString` "Rechte Bildschirmhälfte")
            (if true
              _)))))))

(event `InputAxis|Left/Right`
  (params (AxisValue :type "Float (single-precision)"))
  ;[0 1 0.5961 1 200] WASD or Arrow Keys Movement
  (`self.AddMovementInput` (`KismetMathLibrary.GetRightVector` (`KismetMathLibrary.MakeRotator` 0.0 0.0 (.yaw (`self.GetControlRotation`)))) AxisValue))

(fn `CalculateSpeed`)

(fn `CheckIfTouchOnCharacter`
  ;[1 0 0] Not working yet // Check if Touch Input is On The Cat Character itself
  (`KismetSystemLibrary.PrintString` (`KismetStringLibrary.Conv_VectorToString` (`GameplayStatics.DeprojectScreenToWorld` (`GameplayStatics.GetPlayerController` 0) (0.0 0.0)))))

(fn `SetHorizontalSwipeSpeed`
  (set `CharacterMovementComponent.MaxAcceleration` (`/Game/Multitascats/Core/GameInstance/BP_GameInstance.horizontalSwipeSpeed` (`self.GameInstance_REF`)) (`self.CharacterMovement`)))

(fn `UserConstructionScript`)